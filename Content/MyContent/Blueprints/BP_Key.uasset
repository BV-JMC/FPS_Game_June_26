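; BP_Key is a pickup that stays hidden and without collision until no BP_Target actors remain in the level.
; Tick polls the target count each frame to toggle visibility and collision, playing a one-time Niagara effect and sound when the key appears.
; Overlap by the cached first-person player then sets its HasKey flag, plays a collect sound and destroys the key.
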(event OnComponentBeginOverlap(Collision)
  (params (OverlappedComponent :type Primitive%20Component%20Object%20Reference) (OtherActor :type Actor%20Object%20Reference) (OtherComp :type Primitive%20Component%20Object%20Reference) (OtherBodyIndex :type Integer) (bFromSweep :type Boolean) (SweepResult :type Hit%20Result%20Structure%20%28by%20ref%29))
  ;[0.15 0.15 0.15 0.5] Collecting the Key
  (if (and (== OtherActor (Variables|Default|GetPlayerRef)) (Variables|Default|GetAllTargetsDestroyed))
    (Variables|/Game/StarterContent/FirstPerson/Blueprints/BP_FirstPersonCharacter.BP_FirstPersonCharacter_C|SetHasKey (Variables|Default|GetPlayerRef) true)
    (Audio|PlaySoundatLocation "/Game/MyContent/Audio/MP3_Key_Collect.MP3_Key_Collect" (Transformation|GetActorLocation) "0, 0, 0" 1.0 1.0 0.0 0 0 0 0)
    (Actor|DestroyActor)))

(event EventBeginPlay
  ;[0.15 0.15 0.15 0.5] Setup
  (bind _asbp_first_person_character (Utilities|Casting|CastToBP_FirstPersonCharacter (Game|GetPlayerCharacter 0)))
  (Variables|Default|SetPlayerRef _asbp_first_person_character))

(event EventTick
  (params (DeltaSeconds :type Float%20%28single-precision%29))
  (bind _sm_key (Variables|Default|GetSM_Key))
  (bind _returnvalue (Transformation|GetWorldLocation _sm_key))
  ;[0.15 0.15 0.15 0.5] Key Visibility
  (bind _outactors (Actor|GetAllActorsOfClass "/Game/MyContent/Blueprints/BP_Target.BP_Target_C"))
  (bind _returnvalue_2 (Utilities|Array|Add _outactors 0))
  (bind _output_get (Variables|Default|SetAllTargetsDestroyed (<= _returnvalue_2 0)))
  (Rendering|SetVisibility (Variables|Default|GetSM_Key) _output_get false)
  (Collision|SetActorEnableCollision _output_get)
  ;[0.15 0.15 0.15 0.5] Collect Effects
  (if (Variables|Default|GetAllTargetsDestroyed)
    (Utilities|FlowControl|DoOnce false
      (:Completed
        (Niagara|SpawnSystematLocation "/Game/MyContent/FX/PE_KeyAppear.PE_KeyAppear" _returnvalue)
        (Audio|SpawnSoundatLocation "/Game/MyContent/Audio/MP3_Key_Appear.MP3_Key_Appear" _returnvalue "0, 0, 0" 1.0 1.0 0.0 0 0)))))

(fn ConstructionScript)