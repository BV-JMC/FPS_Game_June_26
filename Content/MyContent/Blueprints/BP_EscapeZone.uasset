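; BP_EscapeZone is a trigger volume that marks the point where the player escapes.
; On BeginPlay it caches the first player's BP_FirstPersonCharacter as a reference.
; When that character begins overlapping its Collision component, it sets the character's Escaped flag and disables the player's input.
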(event OnComponentBeginOverlap(Collision)
  (params (OverlappedComponent :type Primitive%20Component%20Object%20Reference) (OtherActor :type Actor%20Object%20Reference) (OtherComp :type Primitive%20Component%20Object%20Reference) (OtherBodyIndex :type Integer) (bFromSweep :type Boolean) (SweepResult :type Hit%20Result%20Structure%20%28by%20ref%29))
  (bind _playerref (Variables|Default|GetPlayerRef))
  ;[0.15 0.15 0.15 0.5] Player has entered the collision
  (if (== OtherActor _playerref)
    (Variables|/Game/StarterContent/FirstPerson/Blueprints/BP_FirstPersonCharacter.BP_FirstPersonCharacter_C|SetEscaped _playerref true)
    (Input|DisableInput (Variables|Default|GetPlayerRef) (Game|GetPlayerController 0))))

(event EventBeginPlay
  (bind _asbp_first_person_character (Utilities|Casting|CastToBP_FirstPersonCharacter (Game|GetPlayerCharacter 0)))
  (Variables|Default|SetPlayerRef _asbp_first_person_character))

(fn ConstructionScript)